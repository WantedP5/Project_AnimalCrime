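; BP_VoiceTestCharacter is a test character that sets up positional VOIP voice chat.
; On BeginPlay it adds a VOIP Talker, polls with a short delay until PlayerState is valid, then registers the talker with it.
; It then sets the mic threshold and attaches voice to the capsule using SA_VOIP attenuation.
; Console-command nodes for voice loopback and toggling speech are left unconnected.
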(event `self.ReceiveBeginPlay`
  (bind _playerstate (`self.PlayerState`))
  (bind _returnvalue (`AddComponent|NODE_AddVOIPTalker-0`))
  (set `self.VOIP REF` _returnvalue)
  (`/Engine/EditorBlueprintResources/StandardMacros.IsValid` _playerstate :!label _label
    (:`Is Valid`
      (`VOIPTalker.RegisterWithPlayerState` (`self.VOIP REF`) _playerstate)
      (`VOIPStatics.SetMicThreshold` -1.0)
      (set `VOIPTalker.Settings` (make `VoiceSettings` (`self.CapsuleComponent`) "/Game/Project/Sound/SA_VOIP.SA_VOIP") (`self.VOIP REF`))
      (if (`self.IsLocallyControlled`)
        _))
    (:`Is Not Valid`
      (`KismetSystemLibrary.Delay` 0.2)
      (goto _label))))

(fn `UserConstructionScript`)