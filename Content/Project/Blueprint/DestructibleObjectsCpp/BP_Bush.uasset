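; BP_Bush is a destructible bush whose destruction earns game score as a Mafia DestroyObject action.
; Damage feeds its DestroyableStat component, printing remaining HP until it reaches zero, then calls ServerOnDestroyByPlayer.
; The server destroy event passes the stat's score points to ACMainGameMode, prints the total score and destroys the actor.
; Actor overlap events only toggle OverlapFlag, which nothing in the graph reads.
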(event `self.ReceiveActorBeginOverlap`
  (params (OtherActor :type "Actor Object Reference"))
  ; 미구현
  (set `self.bOverlapFlag` true))

(event `self.ReceiveActorEndOverlap`
  (params (OtherActor :type "Actor Object Reference"))
  ; 미구현
  (set `self.bOverlapFlag` false))

(event `self.ReceiveAnyDamage`
  (params (Damage :type "Float (single-precision)") (DamageType :type "DamageType Object Reference") (InstigatedBy :type "Controller Object Reference") (DamageCauser :type "Actor Object Reference"))
  (bind _destroyablestat (`self.DestroyableStat`))
  (`ACDestroyableStatComponent.OnDamaged` _destroyablestat Damage)
  (if (<= (`ACDestroyableStatComponent.GetCurrentHp` _destroyablestat) 0.0)
    (`self.Server_OnDestroyByPlayer`)
    (else
      (`KismetSystemLibrary.PrintString` (`KismetStringLibrary.Conv_DoubleToString` (`ACDestroyableStatComponent.GetCurrentHp` (`self.DestroyableStat`)))))))

(event `self.ReceivePointDamage`
  (params (Damage :type "Float (single-precision)") (DamageType :type "DamageType Object Reference") (HitLocation :type "Vector Structure") (HitNormal :type "Vector Structure") (HitComponent :type "PrimitiveComponent Object Reference") (BoneName :type Name) (ShotFromDirection :type "Vector Structure") (InstigatedBy :type "Controller Object Reference") (DamageCauser :type "Actor Object Reference") (HitInfo :type "HitResult Structure (by ref)")))

(event `Server_OnDestroyByPlayer`
  (bind _asacmain_game_mode (cast `ACMainGameMode` (`GameplayStatics.GetGameMode`)))
  (`ACMainGameMode.UpdateGameScoreFromMafia` _asacmain_game_mode "DestroyObject" (`ACDestroyableStatComponent.GetScorePoint` (`self.DestroyableStat`)))
  (`KismetSystemLibrary.PrintString` (`KismetStringLibrary.Conv_IntToString` (`KismetMathLibrary.FTrunc` (`ACMainGameMode.GetGameScore` _asacmain_game_mode))))
  (`self.K2_DestroyActor`))

(fn `UserConstructionScript`)