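; Lobby character Blueprint providing push-to-talk VOIP with positional (hold V) and radio (hold R) voice modes.
; A multicast init retries until PlayerState is valid, then registers the VOIPTalker with it.
; Keys set VoiceMode through the server, and its OnRep applies mesh-attached attenuation or a radio effect chain.
; A client event closes the line by muting talkers and clearing voice packets.
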(event `Multicast_InitVOIIP`
  (`/Engine/EditorBlueprintResources/StandardMacros.IsValid` (`self.PlayerState`) :!label _label
    (:`Is Valid`
      (`AdvancedVoiceLibrary.RemoveAllRemoteTalkers`)
      (`VOIPTalker.RegisterWithPlayerState` (`self.VOIPTalker`) (`self.PlayerState`))
      (`VOIPStatics.SetMicThreshold` -1.5)
      (set `VOIPTalker.Settings` (select `EVoiceMode` (`self.VoiceMode`) :`None` (make `VoiceSettings` null) :`Positional` (make `VoiceSettings` (`self.Mesh`) "/Game/Project/Sound/SA_VOIP.SA_VOIP") :`Radio` (make `VoiceSettings` null null "/Game/Project/Sound/SEPC_Radio.SEPC_Radio")) (`self.VOIPTalker`)))
    (:`Is Not Valid`
      (`KismetSystemLibrary.RetriggerableDelay` 0.2)
      (goto _label))))

(event `Server_SetVoiceMode`
  (params (VoiceMode :type "EVoiceMode Enum" :default "None"))
  (set `self.VoiceMode` VoiceMode))

(event `Client_CloseVoiceLine`
  (`self.VOIPTalker`
    (:`then`
      (if (`|EnumInequality` (`self.VoiceMode`))
        (`KismetSystemLibrary.ExecuteConsoleCommand` "ToggleSpeaking 0" (`PlayerState.GetPlayerController` (`self.PlayerState`))))
      (`AdvancedVoiceLibrary.MuteRemoteTalker` 0 (`AdvancedSessionsLibrary.GetUniqueNetIDFromPlayerState` (`self.PlayerState`)) true)
      (`AdvancedVoiceLibrary.RemoveAllRemoteTalkers`)
      (`ACVOIPLibrary.ClearVoicePackets` self))
    (:`else`)))

(event `Key|V`
  (params (Key :type "Key Structure"))
  (:`Pressed`
    (`self.VOIPTalker`
      (:`then`
        (`self.Server_SetVoiceMode` "Positional")
        (`AdvancedVoiceLibrary.StartNetworkedVoice` 0))
      (:`else`)))
  (:`Released`
    (`AdvancedVoiceLibrary.StopNetworkedVoice` 0)
    (`self.Server_SetVoiceMode` "None")))

(event `Key|R`
  (params (Key :type "Key Structure"))
  (:`Pressed`
    (`self.VOIPTalker`
      (:`then`
        (`self.Server_SetVoiceMode` "Radio")
        (`AdvancedVoiceLibrary.StartNetworkedVoice` 0))
      (:`else`)))
  (:`Released`
    (`AdvancedVoiceLibrary.StopNetworkedVoice` 0)
    (`self.Server_SetVoiceMode` "None")))

(fn `OnRep_VoiceMode`
  (set `VOIPTalker.Settings` (select `EVoiceMode` (`self.VoiceMode`) :`None` (make `VoiceSettings` null) :`Positional` (make `VoiceSettings` (`self.Mesh`) "/Game/Project/Sound/SA_VOIP.SA_VOIP") :`Radio` (make `VoiceSettings` null null "/Game/Project/Sound/SEPC_Radio.SEPC_Radio")) (`self.VOIPTalker`)))

(fn `UserConstructionScript`)